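; Behavior tree task that finds and claims a smart object slot near the controlled NPC pawn.
; It queries the Smart Object subsystem in a box around the pawn for gameplay-behavior smart objects and claims a random result's slot.
; A valid claim handle is written to the blackboard and the task succeeds; no results or an invalid claim fail it.
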(event EventReceiveExecuteAI
  (params (OwnerController :type AI%20Controller%20Object%20Reference) (ControlledPawn :type Pawn%20Object%20Reference))
  (bind _returnvalue (Transformation|GetActorLocation ControlledPawn))
  (Variables|Default|SetBlackboard (Variables|/Script/AIModule.AIController|GetBlackboard OwnerController))
  (bind _outresults (Class|SmartObjectSubsystem|FindSmartObjectsBP (Subsystems|GetSmartObjectSubsystem) (Utilities|Struct|MakeSmartObjectRequest (Math|Box|MakeBox (- _returnvalue "2000.000000,2000.000000,2000.000000") (+ _returnvalue "2000.000000,2000.000000,2000.000000")) (Utilities|Struct|MakeSmartObjectRequestFilter "(GameplayTags=)" "(TokenStreamVersion=0,TagDictionary=,QueryTokenStream=,UserDescription=\"\",AutoDescription=\"\")" (Utilities|Array|MakeArray "/Script/GameplayBehaviorSmartObjectsModule.GameplayBehaviorSmartObjectBehaviorDefinition") true)) 0))
  (bind _output_get (Variables|Default|SetOut%20Results _outresults))
  (if (Utilities|Array|IsNotEmpty _output_get)
    (bind _returnvalue_2 (Class|SmartObjectBlueprintFunctionLibrary|MarkSmartObjectSlotasClaimed (.slothandle (.OutItem (Utilities|Array|Random (Variables|Default|GetOut%20Results)))) 0))
    (bind _output_get_2 (Variables|Default|SetClaimHandle _returnvalue_2))
    (bind _returnvalue_3 (Class|SmartObjectBlueprintFunctionLibrary|IsValidSmartObjectClaimHandle _output_get_2))
    (if _returnvalue_3
      (Class|SmartObjectBlueprintFunctionLibrary|SetValueasSOClaimHandle (Variables|Default|GetBlackboard) (Utilities|Name|MakeLiteralName "SOClaimHandleKey") (Variables|Default|GetClaimHandle))
      (AI|BehaviorTree|FinishExecute true)
      (else
        (AI|BehaviorTree|FinishExecute false)))
    (else
      (AI|BehaviorTree|FinishExecute false))))