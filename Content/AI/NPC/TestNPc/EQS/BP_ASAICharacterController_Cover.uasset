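; AI controller for a test NPC that runs the find-cover behavior tree on BeginPlay.
; Perception updates pass through touch, sight, hearing and prediction handlers, which write TargetActor, TargetLocation and LastKnownLocation to the Blackboard.
; Losing sight of the player requests a one-second pawn prediction but leaves TargetActor on the player, since both select inputs are the player.
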(event OnTargetPerceptionUpdated(AIPerception)
  (params (Actor :type Actor%20Object%20Reference) (Stimulus :type AI%20Stimulus%20Structure))
  (CallFunction|HandleTouchSense Actor Stimulus)
  (CallFunction|HandleSightSense Actor Stimulus)
  (CallFunction|HandleSoundSense Stimulus)
  (CallFunction|HandlePrediction Stimulus))

(event EventBeginPlay
  (AI|RunBehaviorTree "/Game/AI/NPC/TestNPc/EQS/BP_BTFindCover.BP_BTFindCover"))

(event EventTick
  (params (DeltaSeconds :type Float%20%28single-precision%29)))

(fn ConstructionScript)

(fn HandleSightSense
  (params (Actor :type Actor%20Object%20Reference) (Stimulus :type AI%20Stimulus%20Structure))
  (bind _returnvalue (Game|GetPlayerCharacter 0))
  (bind _returnvalue_2 (Class|AIPerceptionSystem|GetSenseClassforStimulus Stimulus))
  (if (== _returnvalue_2 "/Script/AIModule.AISense_Sight")
    (if (== Actor (Game|GetPlayerCharacter 0))
      (AI|Components|Blackboard|SetValueasObject (Variables|Default|GetBlackboard) (Utilities|Name|MakeLiteralName "TargetActor") (Utilities|SelectObject _returnvalue _returnvalue (.bsuccessfullysensed Stimulus)))
      (if (not (.bsuccessfullysensed Stimulus))
        (Class|AISensePrediction|RequestPawnPredictionEvent (Pawn|GetControlledPawn) (Game|GetPlayerCharacter 0) 1.0))
      (else
        (return)))
    (else
      (return))))

(fn HandleSoundSense
  (params (Stimulus :type AI%20Stimulus%20Structure))
  (bind _returnvalue (Class|AIPerceptionSystem|GetSenseClassforStimulus Stimulus))
  (if (== _returnvalue "/Script/AIModule.AISense_Hearing")
    (AI|Components|Blackboard|SetValueasVector (Variables|Default|GetBlackboard) (Utilities|Name|MakeLiteralName "TargetLocation") (.StimulusLocation (Utilities|Struct|BreakAIStimulus Stimulus)))))

(fn HandleTouchSense
  (params (Actor :type Actor%20Object%20Reference) (Stimulus :type AI%20Stimulus%20Structure))
  (bind _returnvalue (Class|AIPerceptionSystem|GetSenseClassforStimulus Stimulus))
  (if (== _returnvalue "/Script/AIModule.AISense_Touch")
    (if (== Actor (Game|GetPlayerCharacter 0))
      (AI|Components|Blackboard|SetValueasObject (Variables|Default|GetBlackboard) (Utilities|Name|MakeLiteralName "TargetActor") (Utilities|SelectObject (Game|GetPlayerCharacter 0) 0 (.bsuccessfullysensed Stimulus)))
      (else
        (return)))
    (else
      (return))))

(fn HandlePrediction
  (params (Stimulus :type AI%20Stimulus%20Structure))
  (bind _returnvalue (Class|AIPerceptionSystem|GetSenseClassforStimulus Stimulus))
  (if (== _returnvalue "/Script/AIModule.AISense_Prediction")
    (AI|Components|Blackboard|SetValueasVector (Variables|Default|GetBlackboard) (Utilities|Name|MakeLiteralName "LastKnownLocation") (.StimulusLocation (Utilities|Struct|BreakAIStimulus Stimulus)))))