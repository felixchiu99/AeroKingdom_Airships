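; BP_AIObject_PatrolPath is an AI patrol point actor that turns a visiting character to face the direction of its Arrow.
; On patroller entry it stores the character, opens a Gate and fires OnPointMet.
; While the Gate is open, Tick smoothly interpolates the character's rotation toward the Arrow's world rotation using RInterpTo, until patroller exit closes the Gate.
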(event Custom|OnPatrollerEntered
  (params (Character :type Character%20Object%20Reference))
  (Variables|Default|SetCharacter Character)
  (Utilities|FlowControl|Sequence
    (:then_0
      (Utilities|FlowControl|Gate true) ; enters at Open
    )
    (:then_1
      (Default|CallOnPointMet))))

(event Custom|OnPatrollerExit
  (bind _character (Variables|Default|GetCharacter))
  (Utilities|FlowControl|Gate true) ; enters at Close
)

(event EventBeginPlay)

(event Collision|EventActorBeginOverlap
  (params (OtherActor :type Actor%20Object%20Reference)))

(event EventTick
  (params (DeltaSeconds :type Float%20%28single-precision%29))
  (bind _character (Variables|Default|GetCharacter))
  (Utilities|FlowControl|Gate true
    (:Exit
      (Transformation|SetActorRotation _character (Math|Interpolation|RInterpTo (Transformation|GetActorRotation _character) (Transformation|GetWorldRotation (Variables|Default|GetArrow)) DeltaSeconds 2.0)))))

(fn ConstructionScript)